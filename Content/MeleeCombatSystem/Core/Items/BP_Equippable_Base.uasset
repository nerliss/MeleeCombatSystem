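; BP_Equippable_Base is a base actor for equippable items in the melee combat system.
; Equipping sets the equipped flag, snaps the item to its attach socket on the owning BP_Player_Character's mesh and disables collision.
; Unequipping clears the flag and restores collision without detaching.
; A mesh getter returns the static mesh component when it has a valid mesh, otherwise the skeletal one.
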(fn `AttachToAnActor`
  (params (SocketName :type Name))
  (`self.K2_AttachToComponent` (`Character.Mesh` (cast `/Game/MeleeCombatSystem/Core/Characters/BP_Player_Character` (`self.GetOwner`) :!pure true)) SocketName "SnapToTarget" "SnapToTarget" "SnapToTarget"))

(fn `GetEquipped`
  (returns (bEquipped :type Boolean))
  (return (`self.bEquipped`)))

(fn `GetItemMesh`
  (returns (MeshPrimitive :type "PrimitiveComponent Object Reference"))
  (`StaticMeshComponent.StaticMesh` (`self.ItemStaticMesh`)
    (:`then`
      (return (`self.ItemStaticMesh`)))
    (:`else`
      (return (`self.ItemSkeletalMesh`)))))

(fn `OnEquipped`
  (set `self.bEquipped` true)
  (`self.AttachToAnActor` (`self.AttachSocketName`))
  (`self.SetActorEnableCollision` false))

(fn `OnUnequipped`
  (if (`self.bEquipped`)
    (set `self.bEquipped` false)
    (`self.SetActorEnableCollision` true)))

(fn `SetEquipped`
  (params (bEquipped :type Boolean))
  (set `self.bEquipped` bEquipped))

(fn `UserConstructionScript`)