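; Base pickup actor for the melee combat system that gives the interacting user an equipped item.
; On Interact it spawns ItemClassToSpawn at its own transform, with the user as owner and instigator, then calls OnEquipped on the spawned item.
; The construction script previews the item by copying static and skeletal meshes from that class's defaults.
; The CanBePickedUp flag answers whether it can be interacted with.
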(event `/Game/MeleeCombatSystem/Core/Interfaces/BPI_Interactable.Interact`
  (params (User :type "/Game/MeleeCombatSystem/Core/Characters/BP_Player_Character Object Reference"))
  (bind _returnvalue (`|SpawnActorFromClass` (`self.ItemClassToSpawn`) (`self.GetTransform`) "AlwaysSpawn" "OverrideRootScale" User User))
  (`/Game/MeleeCombatSystem/Core/Items/BP_Equippable_Base.OnEquipped` _returnvalue))

(fn `CanBeInteractedWith`
  (returns (Return :type Boolean))
  (return (`self.bCanBePickedUp`)))

(fn `UserConstructionScript`
  (bind (_bequipped _attachsocketname _righthandsocket _bcanbeinteractedwith _staticmeshtoset _skeletalmeshtoset) (defaults `Object` (`self.ItemClassToSpawn`)))
  ;[1 1 1] Set preview mesh in runtime
  (`StaticMeshComponent.SetStaticMesh` (`self.ItemStaticMesh`) _staticmeshtoset)
  (`SkinnedMeshComponent.SetSkinnedAssetAndUpdate` (`self.ItemSkeletalMesh`) _skeletalmeshtoset true))