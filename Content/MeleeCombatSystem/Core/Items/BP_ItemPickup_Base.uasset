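; Base world pickup for the melee combat system that shows an item's mesh and gives the item to whoever interacts with it.
; On BeginPlay it spawns the configured item class to copy its static or skeletal mesh, without destroying that instance afterwards.
; Interact spawns a new item owned and instigated by the user and calls OnEquipped, leaving the pickup in place.
; CanBeInteractedWith returns the CanBePickedUp flag.
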(event `self.ReceiveBeginPlay`
  (`|ExecutionSequence`
    (:`then_0`
      ;[1 0 0] TODO: Try and move it to construction script
      (bind _returnvalue (`|SpawnActorFromClass` (`self.ItemClassToSpawn`) (`self.GetTransform`) "AlwaysSpawn" "OverrideRootScale" null null))
      (bind _meshprimitive (`/Game/MeleeCombatSystem/Core/Items/BP_Equippable_Base.GetItemMesh` _returnvalue))
      (bind _asstatic_mesh_component (cast `StaticMeshComponent` _meshprimitive)
        (:`then`
          (`StaticMeshComponent.SetStaticMesh` (`self.ItemStaticMesh`) (`StaticMeshComponent.StaticMesh` _asstatic_mesh_component)))
        (:`CastFailed`
          (bind _asskeletal_mesh_component (cast `SkeletalMeshComponent` _meshprimitive))
          (`SkinnedMeshComponent.SetSkinnedAssetAndUpdate` (`self.ItemSkeletalMesh`) (`SkinnedMeshComponent.SkeletalMesh` _asskeletal_mesh_component) true))))))

(event `/Game/MeleeCombatSystem/Core/Interfaces/BPI_Interactable.Interact`
  (params (User :type "/Game/MeleeCombatSystem/Core/Characters/BP_Player_Character Object Reference"))
  (bind _returnvalue (`|SpawnActorFromClass` (`self.ItemClassToSpawn`) (`self.GetTransform`) "AlwaysSpawn" "OverrideRootScale" User User))
  (`/Game/MeleeCombatSystem/Core/Items/BP_Equippable_Base.OnEquipped` _returnvalue))

(fn `CanBeInteractedWith`
  (returns (Return :type Boolean))
  (return (`self.bCanBePickedUp`)))

(fn `UserConstructionScript`)