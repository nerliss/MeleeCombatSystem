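; BP_CombatCollisionComponent is an actor component that detects hits for melee combat.
; While collision is enabled, it runs a multi-sphere object trace every tick between two sockets on an assigned mesh component.
; Each actor is recorded on first contact and reported through OnHit only once until the list is cleared, which happens whenever collision is enabled.
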(event `self.ReceiveTick`
  (params (DeltaSeconds :type "Float (single-precision)"))
  (if (`self.bCollisionEnabled`)
    (`self.CollisionTrace`)))

(event `EnableCollision`
  (`self.ClearHitActors`)
  (set `self.bCollisionEnabled` true))

(event `DisableCollision`
  (set `self.bCollisionEnabled` false))

(event `ClearHitActors`
  (`KismetArrayLibrary.Array_Clear` (`self.AlreadyHitActors`)))

(event `CollisionTrace`
  (bind _collisionmeshcomponent (`self.CollisionMeshComponent`))
  (bind _alreadyhitactors (`self.AlreadyHitActors`))
  (bind _outhits (`KismetSystemLibrary.SphereTraceMultiForObjects` (`SceneComponent.GetSocketLocation` _collisionmeshcomponent (`self.StartSocketName`)) (`SceneComponent.GetSocketLocation` _collisionmeshcomponent (`self.EndSocketName`)) (`self.TraceRadius`) (`self.CollisionObjectTypes`) false (`self.ActorsToIgnore`) (`self.Draw Debug Type`)))
  (for _array_element _outhits
    (bind _output_get (set `self.LastHit` _array_element))
    (bind (_bblockinghit _binitialoverlap _time _distance _location _impactpoint _normal _impactnormal _physmat _hitactor) (`GameplayStatics.BreakHitResult` _output_get))
    (if (not (`KismetArrayLibrary.Array_Contains` _alreadyhitactors _hitactor))
      (bind _output_get_2 (set `self.Hit Actor` _hitactor))
      (`KismetArrayLibrary.Array_Add` _alreadyhitactors _output_get_2)
      (`self.OnHit` _output_get))))

(fn `GetAlreadyHitActors`
  (returns (AlreadyHitActors :type "Array of Actor Object Reference"))
  (return (`self.AlreadyHitActors`)))

(fn `GetCollisionEnabled`
  (returns (bCollisionEnabled :type Boolean))
  (return (`self.bCollisionEnabled`)))

(fn `GetLastHit`
  (returns (LastHit :type "HitResult Structure"))
  (return (`self.LastHit`)))

(fn `SetCollisionMeshComponent`
  (params (NewCollisionMeshComponent :type "PrimitiveComponent Object Reference"))
  (returns (CollisionMeshComponent :type "PrimitiveComponent Object Reference"))
  (set `self.CollisionMeshComponent` NewCollisionMeshComponent))