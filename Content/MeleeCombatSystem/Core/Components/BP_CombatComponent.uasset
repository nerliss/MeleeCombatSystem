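; Actor component that holds melee combat state for its owner: the main weapon, the in-combat flag and attack tracking.
; Setting a new main weapon first unequips and destroys the current one.
; Changing the in-combat flag forwards it to the player character's mesh anim instance through an update message, casting the owner to BP_Character_Player.
; ResetAttack clears the attack count, saved-attack flag and attacking flag.
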(fn `GetInCombat`
  (returns (bInCombat :type Boolean))
  (return (`self.bInCombat`)))

(fn `GetMainWeapon`
  (returns (MainWeapon :type "/Game/MeleeCombatSystem/Core/Items/Weapons/BP_Weapon_Base Object Reference"))
  (return (`self.MainWeapon`)))

(fn `ResetAttack`
  (set `self.AttackCount` 0)
  (set `self.bAttackSaved` false)
  (set `self.bIsAttacking` false))

(fn `SetInCombat`
  (params (NewInCombat :type Boolean))
  (bind _output_get (set `self.bInCombat` NewInCombat))
  (message `/Game/MeleeCombatSystem/Core/Interfaces/BPI_AnimInstance.UpdateInCombat` (`SkeletalMeshComponent.GetAnimInstance` (`Character.Mesh` (cast `/Game/MeleeCombatSystem/Core/Characters/BP_Character_Player` (`self.GetOwner`) :!pure true))) _output_get))

(fn `SetMainWeapon`
  (params (NewWeapon :type "/Game/MeleeCombatSystem/Core/Items/Weapons/BP_Weapon_Base Object Reference"))
  (`|ExecutionSequence`
    (:`then_0`
      (bind _mainweapon (`self.MainWeapon`)
        (:`then`
          (`/Game/MeleeCombatSystem/Core/Items/BP_Equippable_Base.OnUnequipped` _mainweapon)
          (`Actor.K2_DestroyActor` _mainweapon)
          (set `self.MainWeapon` null))
        (:`else`)))
    (:`then_1`
      (set `self.MainWeapon` NewWeapon))))